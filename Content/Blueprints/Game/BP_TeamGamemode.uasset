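; Team-based game mode that scores kills for teams and spawns players on their own team's starts.
; On a death update, it runs the parent logic, then adds one point to the instigator's team through BP_TeamGameState.
; Spawn selection returns only free BP_GamePlayerStart actors whose team matches the player's BP_TeamPlayerState team.
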(event `self.UpdateDeathPoints`
  (params (Character :type "/Game/Blueprints/Player/BP_PlayerController Object Reference") (Instigator :type "/Game/Blueprints/Player/BP_PlayerController Object Reference"))
  (`parent.UpdateDeathPoints` Character Instigator)
  (`/Game/Blueprints/Game/BP_TeamGameState.ChangeTeamPoint` (cast `/Game/Blueprints/Game/BP_TeamGameState` (`GameplayStatics.GetGameState`) :!pure true) (`/Game/Blueprints/Player/BP_TeamPlayerState.Team` (cast `/Game/Blueprints/Player/BP_TeamPlayerState` (`Controller.PlayerState` Instigator) :!pure true)) 1))

(fn `GetFreeSpawnPoints`
  (params (Player :type "/Game/Blueprints/Player/BP_PlayerController Object Reference"))
  (returns (FreeSpawns :type "Array of /Game/Blueprints/Game/BP_GamePlayerStart Object Reference"))
  (locals (L_FreePoints :type "Array of /Game/Blueprints/Game/BP_GamePlayerStart Object Reference"))
  (bind _outactors (`GameplayStatics.GetAllActorsOfClass` "/Game/Blueprints/Game/BP_GamePlayerStart.BP_GamePlayerStart_C"))
  (for _array_element _outactors
    (if (and (`/Game/Blueprints/Game/BP_GamePlayerStart.IsFree` _array_element) (`|EnumEquality` (`/Game/Blueprints/Player/BP_TeamPlayerState.Team` (cast `/Game/Blueprints/Player/BP_TeamPlayerState` (`Controller.PlayerState` Player) :!pure true)) (`/Game/Blueprints/Game/BP_GamePlayerStart.Team` _array_element)))
      (`KismetArrayLibrary.Array_Add` (`local.L_FreePoints`) _array_element)))
  (return (`local.L_FreePoints`)))

(fn `UserConstructionScript`
  (`parent.UserConstructionScript`))