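; BP_BaseGamemode is a base game mode Blueprint that handles player spawning and character death notifications.
; SpawnPlayer gathers every BP_GamePlayerStart reporting itself free, picks one at random and has it spawn the player's character.
; CharacterDead relays the dead character, instigator and cause through CallCharDead.
; The construction script and NewFunction_0 are empty.
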(fn `CharacterDead`
  (params (DeadCharacter :type "/Game/Blueprints/Player/BP_PlayerCharacter Object Reference") (DeathInstigator :type "/Game/Blueprints/Player/BP_PlayerController Object Reference") (DeathCauseBy :type "Actor Object Reference"))
  (`self.CharDead` DeadCharacter DeathInstigator DeathCauseBy))

(fn `GetFreeSpawnPoints`
  (returns (FreeSpawns :type "Array of /Game/Blueprints/Game/BP_GamePlayerStart Object Reference"))
  (locals (L_FreePoints :type "Array of /Game/Blueprints/Game/BP_GamePlayerStart Object Reference"))
  (bind _outactors (`GameplayStatics.GetAllActorsOfClass` "/Game/Blueprints/Game/BP_GamePlayerStart.BP_GamePlayerStart_C"))
  (for _array_element _outactors
    (if (`/Game/Blueprints/Game/BP_GamePlayerStart.IsFree` _array_element)
      (`KismetArrayLibrary.Array_Add` (`local.L_FreePoints`) _array_element)))
  (return (`local.L_FreePoints`)))

(fn `NewFunction_0`
  (params (self2 :type "/Game/Blueprints/Game/BP_GamePlayerStart Object Reference")))

(fn `SpawnPlayer`
  (params (Player :type "/Game/Blueprints/Player/BP_PlayerController Object Reference"))
  (locals (L_PlayerStart :type "/Game/Blueprints/Game/BP_GamePlayerStart Object Reference"))
  (bind _freespawns (`self.GetFreeSpawnPoints`))
  (bind _output_get (set `local.L_PlayerStart` (`|GetArrayItem` _freespawns (`KismetMathLibrary.RandomInteger` (`KismetArrayLibrary.Array_LastIndex` _freespawns)))))
  (`/Game/Blueprints/Game/BP_GamePlayerStart.SpawnCharacter` _output_get Player))

(fn `UserConstructionScript`)