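; BP_GamePlayerStart is a player spawn point that creates and tracks a BP_PlayerCharacter standing on it.
; SpawnCharacter spawns the character at its transform, has the player possess it, stores it as the occupant and broadcasts CharacterSpawned.
; Capsule overlap events set or clear that single occupant reference, which IsFree checks to report whether the spot is available.
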(event `self.CapsuleComponent.OnComponentEndOverlap`
  (params (OverlappedComponent :type "PrimitiveComponent Object Reference") (OtherActor :type "Actor Object Reference") (OtherComp :type "PrimitiveComponent Object Reference") (OtherBodyIndex :type Integer))
  (if (== OtherActor (`self.CharecterInside`))
    (set `self.CharecterInside` null)))

(event `self.CapsuleComponent.OnComponentBeginOverlap`
  (params (OverlappedComponent :type "PrimitiveComponent Object Reference") (OtherActor :type "Actor Object Reference") (OtherComp :type "PrimitiveComponent Object Reference") (OtherBodyIndex :type Integer) (bFromSweep :type Boolean) (SweepResult :type "HitResult Structure (by ref)"))
  (bind _asbp_player_character (cast `/Game/Blueprints/Player/BP_PlayerCharacter` OtherActor))
  (set `self.CharecterInside` _asbp_player_character))

(fn `IsFree`
  (returns (Free :type Boolean))
  (`/Engine/EditorBlueprintResources/StandardMacros.IsValid` (`self.CharecterInside`)
    (:`Is Valid`
      (return false))
    (:`Is Not Valid`
      (return true))))

(fn `SpawnCharacter`
  (params (Player :type "/Game/Blueprints/Player/BP_PlayerController Object Reference"))
  (returns (Charecter :type "/Game/Blueprints/Player/BP_PlayerCharacter Object Reference"))
  (bind _returnvalue (`|SpawnActorFromClass` "/Game/Blueprints/Player/BP_PlayerCharacter.BP_PlayerCharacter_C" (`self.GetTransform`) "Undefined" "OverrideRootScale" Player null))
  (bind _output_get (set `self.CharecterInside` _returnvalue))
  (`Controller.Possess` Player _output_get)
  (`self.CharacterSpawned` _output_get Player)
  (return _output_get))

(fn `UserConstructionScript`)