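; Base game state that tracks a round's phase, pre-start countdown and elapsed time for the game mode's rounds.
; On the server, a once-per-second Tick counts down to call StartRound, then advances round time and reports when the time limit is reached.
; The game mode's round-end event is multicast as a dispatcher call, while round start is raised through the phase's OnRep.
; The round-start binding is never run.
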(event `self.ReceiveBeginPlay`
  (`/Engine/EditorBlueprintResources/ActorMacros.Switch Has Authority`
    (:`Authority`
      (add `/Game/Blueprints/Game/BP_BaseGamemode.RoundEnded` (`/Game/Blueprints/Libs/Function/BP_Functions_GlobalGetters.GetGamemode`) (delegate `RoundEnded_Event_0`)))))

(event `RoundEnded_Event_0`
  (params (Reason :type String))
  (`self.Multicast-RoundEnd` Reason)
  (set `self.RoundInProgress` "NewEnumerator2"))

(event `Multicast-RoundEnd`
  (params (Reason :type String))
  (`self.RoundEnded` Reason))

(event `RoundStarted_Event_0`
  (set `self.RoundInProgress` "NewEnumerator0"))

(event `self.ReceiveTick`
  (params (DeltaSeconds :type "Float (single-precision)"))
  (`/Engine/EditorBlueprintResources/ActorMacros.Switch Has Authority`
    (:`Authority`
      (switch `/Game/Data/Enums/E_GameState` (`self.RoundInProgress`)
        (:`NewEnumerator0`
          (bind _result (`/Engine/EditorBlueprintResources/StandardMacros.DecrementInt` (`self.RoundStartTime`))
            (:`  `
              (if (<= _result 0)
                (`/Game/Blueprints/Game/BP_BaseGamemode.StartRound` (`/Game/Blueprints/Libs/Function/BP_Functions_GlobalGetters.GetGamemode`))
                (set `self.RoundInProgress` "NewEnumerator1")))))
        (:`NewEnumerator1`
          (`self.RoundTimeTick`))))))

(fn `GetPreRoundTime`
  (returns (Second :type Integer))
  (return (`self.RoundStartTime`)))

(fn `GetRoundTime`
  (returns (Minute :type Integer) (Second :type Integer))
  (return (`self.CurrentMinute`) (`self.CurrentSecond`)))

(fn `OnRep_RoundInProgress`
  (switch `/Game/Data/Enums/E_GameState` (`self.RoundInProgress`)
    (:`NewEnumerator1`
      (`self.RoundStarted`))))

(fn `RoundTimeTick`
  (bind _output_get (set `self.RoundTime` (+ (`self.RoundTime`) (`KismetMathLibrary.MakeTimespan` 0 0 0 1)))) ; +1 second to round time - +1 секунда к времени раунда
  (bind (_days _hours _minutes _seconds) (`KismetMathLibrary.BreakTimespan` _output_get))
  (set `self.CurrentMinute` _minutes)
  (set `self.CurrentSecond` _seconds)
  (if (and (>= (`self.RoundTime`) (`/Game/Blueprints/Game/BP_BaseGamemode.TimeLimit` (`/Game/Blueprints/Libs/Function/BP_Functions_GlobalGetters.GetGamemode`))) (`|EnumEquality` (`self.RoundInProgress`) "NewEnumerator1"))
    (`/Game/Blueprints/Game/BP_BaseGamemode.TimeLimitReached` (`/Game/Blueprints/Libs/Function/BP_Functions_GlobalGetters.GetGamemode`))))

(fn `StartRoundTimer`
  (bind _returnvalue (`KismetSystemLibrary.K2_SetTimer` null "RoundTimeTick" 1.0 true))
  (set `self.TimeTickTimer` _returnvalue))

(fn `UserConstructionScript`)