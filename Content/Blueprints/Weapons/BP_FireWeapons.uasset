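; BP_FireWeapons is a firearm Blueprint that extends a parent weapon with hitscan firing, ammo and reloading.
; When the parent UseWeapon succeeds, it line-traces from the player camera along the owner's forward vector and debug-draws the hit, without applying damage.
; An empty magazine with reserve ammo sets Reloading, whose RepNotify starts an authority-only timer.
; That timer restores CurrentAmmo from class defaults and deducts the reserve.
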(event `DEBUG_DrawServerTrace`
  (params (Start :type "Vector Structure") (End :type "Vector Structure") (Hit :type "Vector Structure"))
  (`KismetSystemLibrary.DrawDebugLine` Start End (struct) 5.0 2.0)
  (`KismetSystemLibrary.DrawDebugSphere` Hit 40.0 8 (struct :`R` 1.0 :`G` 0.508637 :`A` 1.0) 5.0 2.0))

(fn `AbleToReload`
  (returns (ReturnValue :type Boolean))
  (return (and (!= (defaults `/Game/Blueprints/Weapons/BP_FireWeapons` (`GameplayStatics.GetObjectClass` self)) (`self.CurrentAmmo`)) (> (`self.TotalAmmo`) 0) (not (`KismetSystemLibrary.K2_IsValidTimerHandle` (`self.ReloadTimer`))))))

(fn `GetFireTrace`
  (returns (Hit :type "HitResult Structure"))
  (bind _asbp_player_character (cast `/Game/Blueprints/Player/BP_PlayerCharacter` (`self.GetInstigator`))
    (:`then`
      (bind _returnvalue (`SceneComponent.K2_GetComponentLocation` (`/Game/Blueprints/Player/BP_PlayerCharacter.Camera` _asbp_player_character)))
      (bind _outhit (`KismetSystemLibrary.LineTraceSingle` _returnvalue (+ _returnvalue (* (`self.GetActorForwardVector` (`self.GetOwner`)) 10000.0)) "TraceTypeQuery1" false (`|MakeArray` self (`self.GetInstigator`) :!type "Actor Object Reference")))
      (bind (_bblockinghit _binitialoverlap _time _distance _location _impactpoint _normal _impactnormal _physmat _hitactor _hitcomponent _hitbonename _hititem _faceindex _tracestart _traceend) (`GameplayStatics.BreakHitResult` _outhit))
      (`self.DEBUG_DrawServerTrace` _tracestart _traceend _location)
      (return _outhit))
    (:`CastFailed`
      (return))))

(fn `OnRep_Reloading`
  (`/Engine/EditorBlueprintResources/ActorMacros.Switch Has Authority`
    (:`Authority`
      (if (`self.Reloading`)
        (if (`self.AbleToReload`)
          (`/Game/Blueprints/Libs/BP_Functions_Debug.PrintMessage` "Reloading" (struct :`G` 1.0 :`B` 0.966702 :`A` 1.0) 2.0)
          (bind _returnvalue (`KismetSystemLibrary.K2_SetTimer` null "ReloadFinished" (`self.ReloadTime`)))
          (set `self.ReloadTimer` _returnvalue)
          (set `self.AmmoToReload` (`KismetMathLibrary.Min` (- (defaults `/Game/Blueprints/Weapons/BP_FireWeapons` (`GameplayStatics.GetObjectClass` self)) (`self.CurrentAmmo`)) (`self.TotalAmmo`)))
          (else
            (set `self.Reloading` false)
            (`/Game/Blueprints/Libs/BP_Functions_Debug.PrintMessage` "Not able to reload" (struct :`G` 1.0 :`B` 0.966702 :`A` 1.0) 2.0 true)))))))

(fn `ReloadFinished`
  (set `self.Reloading` false)
  (set `self.CurrentAmmo` (defaults `/Game/Blueprints/Weapons/BP_FireWeapons` (`GameplayStatics.GetObjectClass` self)))
  (set `self.TotalAmmo` (- (`self.TotalAmmo`) (`self.AmmoToReload`))))

(fn `UserConstructionScript`
  (`parent.UserConstructionScript`))

(fn `UseWeapon`
  (returns (used :type Boolean))
  (bind _used (`parent.UseWeapon`))
  (`/Game/Blueprints/Libs/BP_Functions_Debug.PrintMessage` (`KismetStringLibrary.Concat_StrStr` (`KismetStringLibrary.Conv_IntToString` (`self.CurrentAmmo`)) "/" (`KismetStringLibrary.Conv_IntToString` (`self.TotalAmmo`))) (struct :`G` 0.02428 :`B` 0.458333 :`A` 1.0) 1.0)
  (if _used
    (`self.GetFireTrace`)
    (return true)
    (elif (and (<= (`self.CurrentAmmo`) 0) (> (`self.TotalAmmo`) 0))
      (set `self.Reloading` true)
      (return false)
      (else
        (return false)))))