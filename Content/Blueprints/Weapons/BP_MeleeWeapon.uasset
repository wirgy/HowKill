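; BP_MeleeWeapon is a melee weapon that deals point damage to what a short sphere sweep hits.
; Use is blocked while the rate freeze flag is set, and UseWeapon proceeds only if the parent implementation succeeds.
; The sweep starts at the instigating player character's camera and extends along the owner's forward vector by Radius, ignoring weapon and instigator.
; The hit result feeds ApplyPointDamage, with direction pointing from trace end to start.
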(fn `AbleToUseWeapon`
  (returns (Out :type Boolean))
  (return (not (`self.UseFreezedByRate`))))

(fn `GetOverLapInfo`
  (returns (Hit :type "HitResult Structure"))
  (bind _asbp_player_character (cast `/Game/Blueprints/Player/BP_PlayerCharacter` (`self.GetInstigator`))
    (:`then`
      (bind _returnvalue (`SceneComponent.K2_GetComponentLocation` (`/Game/Blueprints/Player/BP_PlayerCharacter.Camera` _asbp_player_character)))
      (bind _outhit (`KismetSystemLibrary.SphereTraceSingleForObjects` _returnvalue (+ _returnvalue (* (`self.GetActorForwardVector` (`self.GetOwner`)) (`self.Radius`))) 30.0 (`|MakeArray` "ObjectTypeQuery1" "ObjectTypeQuery2" "ObjectTypeQuery3" :!type "EObjectTypeQuery Enum") false (`|MakeArray` self (`self.GetInstigator`) :!type "Actor Object Reference")))
      (return _outhit))
    (:`CastFailed`
      (return))))

(fn `UserConstructionScript`
  (`parent.UserConstructionScript`))

(fn `UseWeapon`
  (returns (used :type Boolean))
  (bind _used (`parent.UseWeapon`))
  (if _used
    (bind _hit (`self.GetOverLapInfo`))
    (bind (_bblockinghit _binitialoverlap _time _distance _location _impactpoint _normal _impactnormal _physmat _hitactor _hitcomponent _hitbonename _hititem _faceindex _tracestart _traceend) (`GameplayStatics.BreakHitResult` _hit))
    (`GameplayStatics.ApplyPointDamage` _hitactor (`self.Damage`) (`KismetMathLibrary.GetDirectionUnitVector` _traceend _tracestart) _hit (`self.GetInstigatorController`) self)
    (return true)
    (else
      (return false))))