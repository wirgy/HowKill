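; Base replicated weapon actor that players pick up through Interact, which adds it to their weapon manager.
; UseWeapon spends ammo and starts a use-rate cooldown timer, which re-fires while auto fire stays active.
; WeaponOwner's RepNotify sets ownership and disables collision, attaching to the owner actor on authority, while remotes attach the current weapon to the visible mesh socket and hide others.
; Clearing the owner detaches, unhides and restores collision.
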(fn `AbleToUseWeapon`
  (returns (Out :type Boolean))
  (return (and (> (`self.CurrentAmmo`) 0) (not (`self.UseFreezedByRate`)))))

(fn `interact`
  (params (PlayerCharacter :type "/Game/Blueprints/Player/BP_PlayerCharacter Object Reference"))
  (returns (Success :type Boolean))
  (`/Game/Blueprints/Components/Player/BP_WeaponManager.AddWeapon` (`/Game/Blueprints/Player/BP_PlayerCharacter.BP_WeaponManager` PlayerCharacter) self)
  (return true))

(fn `OnRep_WeaponOwner`
  (bind _weaponowner (`self.WeaponOwner`)
    (:`then`
      (bind _output_get (set `self.Instigator` _weaponowner))
      (`self.SetOwner` (`Pawn.GetController` _output_get))
      (`self.SetActorEnableCollision` false)
      (`/Engine/EditorBlueprintResources/ActorMacros.Switch Has Authority`
        (:`Authority`
          (`self.K2_AttachToActor` (`self.WeaponOwner`) "None" "SnapToTarget" "SnapToTarget" "KeepRelative")
          (`self.SetReplicateMovement` true))
        (:`Remote`
          (if (not (== (`/Game/Blueprints/Components/Player/BP_WeaponManager.CurrentWeapon` (`/Game/Blueprints/Player/BP_PlayerCharacter.BP_WeaponManager` (`self.WeaponOwner`))) self))
            (`self.SetActorHiddenInGame` true)
            (else
              (`self.K2_AttachToComponent` (`/Game/Blueprints/Player/BP_PlayerCharacter.GetVisibleMesh` (`self.WeaponOwner`)) "Skt_Weapon" "SnapToTarget" "SnapToTarget" "KeepRelative"))))))
    (:`else`
      (`self.SetReplicateMovement` true)
      (`self.K2_DetachFromActor` "KeepRelative")
      (`self.SetActorHiddenInGame` false)
      (`self.SetActorEnableCollision` true))))

(fn `StopRateDelay`
  (set `self.UseFreezedByRate` false)
  (if (and (`self.AutoFire`) (`self.FireActive`))
    (`self.UseWeapon`)))

(fn `StopUseWeapon`
  (set `self.FireActive` false))

(fn `UserConstructionScript`)

(fn `UseWeapon`
  (returns (used :type Boolean))
  (if (`self.AbleToUseWeapon`)
    (`/Engine/EditorBlueprintResources/StandardMacros.DecrementInt` (`self.CurrentAmmo`)
      (:`  `
        (`KismetSystemLibrary.K2_SetTimer` null "StopRateDelay" (`self.UseRate`))
        (set `self.UseFreezedByRate` true)
        (if (`self.AutoFire`)
          (set `self.FireActive` true))
        (return true)))
    (else
      (set `self.FireActive` false)
      (return false))))