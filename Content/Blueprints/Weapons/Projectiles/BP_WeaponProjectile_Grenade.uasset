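; BP_WeaponProjectile_Grenade is a thrown physics grenade projectile that explodes after a timed delay.
; On BeginPlay, the authority launches its box with a forward impulse and random spin, then starts the Explode timer.
; Explode applies full radial damage, blocked on WorldStatic, and destroys the actor; remote copies spawn the explosion emitter when destroyed.
; An ignore-list filter sits unused, as a note places damage filtering in the health component.
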(event `self.ReceiveBeginPlay`
  (`/Engine/EditorBlueprintResources/ActorMacros.Switch Has Authority`
    (:`Authority`
      (`PrimitiveComponent.AddImpulse` (`self.Box`) (* (`self.GetActorForwardVector`) (`self.ThrowPower`)) "None" false)
      (`PrimitiveComponent.AddAngularImpulseInRadians` (`self.Box`) (`KismetMathLibrary.MakeVector` (`KismetMathLibrary.RandomFloatInRange` -1000.0 1000.0) (`KismetMathLibrary.RandomFloatInRange` -1000.0 1000.0) (`KismetMathLibrary.RandomFloatInRange` -1000.0 1000.0)) "None" false)
      (`KismetSystemLibrary.K2_SetTimer` null "Explode" (`self.ExplotionDelay`)))))

(event `self.ReceiveDestroyed`
  (`parent.ReceiveDestroyed`)
  (`/Engine/EditorBlueprintResources/ActorMacros.Switch Has Authority`
    (:`Remote`
      (`GameplayStatics.SpawnEmitterAtLocation` "/Game/SciFiWeapLight/FX/Particles/P_Grenade_Explosion_Dark.P_Grenade_Explosion_Dark" (`self.K2_GetActorLocation`)))))

(fn `Explode`
  (locals (L_Ignore :type "Array of Actor Object Reference"))
  (`GameplayStatics.ApplyRadialDamage` :`BaseDamage` (`self.Damage`) :`Origin` (`self.K2_GetActorLocation`) :`DamageRadius` (`self.Explosion Radius`) :`DamageCauser` self :`InstigatedByController` (`self.GetInstigatorController`) :`bDoFullDamage` true :`DamagePreventionChannel` "ECC_WorldStatic")
  (`self.K2_DestroyActor`))

(fn `UserConstructionScript`
  (`parent.UserConstructionScript`))