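; BP_Special_LandMine is a land mine special weapon that explodes when a player character walks into its trigger box.
; On the server, the box overlap asks the game mode whether the instigator may damage that player, and only then detonates.
; Explode applies full radial damage just above the mine's location, blocked by world static geometry, then destroys the actor.
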(event `self.Box.OnComponentBeginOverlap`
  (params (OverlappedComponent :type "PrimitiveComponent Object Reference") (OtherActor :type "Actor Object Reference") (OtherComp :type "PrimitiveComponent Object Reference") (OtherBodyIndex :type Integer) (bFromSweep :type Boolean) (SweepResult :type "HitResult Structure (by ref)"))
  (`/Engine/EditorBlueprintResources/ActorMacros.Switch Has Authority`
    (:`Authority`
      (bind _asbp_player_character (cast `/Game/Blueprints/Player/BP_PlayerCharacter` OtherActor))
      (if (`/Game/Blueprints/Game/BP_BaseGamemode.ShouldDamagePlayer` (`/Game/Blueprints/Libs/Function/BP_Functions_GlobalGetters.GetGamemode`) (`/Game/Blueprints/Libs/Function/BP_Functions_GlobalGetters.GetCharactersController` _asbp_player_character) (cast `/Game/Blueprints/Player/BP_PlayerController` (`self.GetInstigatorController`) :!pure true))
        (`self.Explode`)))))

(fn `Explode`
  (`GameplayStatics.ApplyRadialDamage` :`BaseDamage` (`self.Damage`) :`Origin` (+ (`self.K2_GetActorLocation`) (0.0 0.0 2.0)) :`DamageRadius` (`self.Explosion Radius`) :`DamageCauser` self :`InstigatedByController` (`self.GetInstigatorController`) :`bDoFullDamage` true :`DamagePreventionChannel` "ECC_WorldStatic")
  (`self.K2_DestroyActor`))

(fn `UserConstructionScript`)