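; BP_PlayerState is the player state that tracks a player's alive status, kill count and death count.
; When the owning character dies, it clears Alive and calls PlayerDead with the instigator, death causer and itself.
; The rep notify on Alive calls PlayerAlive when the value becomes true, and simple functions increment Kills and Deaths.
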(event `OwnerCharDead`
  (params (Instigator :type "/Game/Blueprints/Player/BP_PlayerCharacter Object Reference") (DeathCauser :type "Actor Object Reference"))
  (set `self.Alive` false)
  (`self.PlayerDead` Instigator DeathCauser self))

(fn `AddDeath`
  (`/Engine/EditorBlueprintResources/StandardMacros.IncrementInt` (`self.Deaths`)))

(fn `AddKill`
  (`/Engine/EditorBlueprintResources/StandardMacros.IncrementInt` (`self.Kills`)))

(fn `OnRep_Alive`
  (if (`self.Alive`)
    (`self.PlayerAlive`)))

(fn `UserConstructionScript`)