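; Player health component that tracks health and armor and reports the owning character's death to the game mode.
; On the server it binds to the character's damage event, where math expressions scale damage down by current armor and wear armor away with each hit.
; At zero health it flags the character dead once and passes the instigating controller and damage causer to BP_BaseGamemode.
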(event Custom|OnPlayerTakeAnyDamage
  (params (DamagedActor :type Actor%20Object%20Reference) (Damage :type Float%20%28single-precision%29) (DamageType :type Damage%20Type%20Object%20Reference) (InstigatedBy :type Controller%20Object%20Reference) (DamageCauser :type Actor%20Object%20Reference))
  (CallFunction|ApplyDamage Damage)
  (if (and (<= (Variables|Default|GetHealth) 0.0) (not (Variables|/Game/Blueprints/Player/BP_PlayerCharacter.BP_PlayerCharacter_C|GetDead (Variables|Default|GetCharacter))))
    (Variables|/Game/Blueprints/Player/BP_PlayerCharacter.BP_PlayerCharacter_C|SetDead (Variables|Default|GetCharacter) true)
    (bind _asbp_base_gamemode (Utilities|Casting|CastToBP_BaseGamemode (Game|GetGameMode)))
    (Default|CharacterDead _asbp_base_gamemode (Variables|Default|GetCharacter) (.AsBP%20Player%20Controller (Utilities|Casting|CastToBP_PlayerController InstigatedBy)) DamageCauser)))

(event EventBeginPlay
  (Variables|Default|SetHealth (Variables|Default|GetMaxHealth))
  (Variables|Default|SetArmor (Variables|Default|GetMaxArmor))
  (bind _asbp_player_character (Utilities|Casting|CastToBP_PlayerCharacter (Components|GetOwner)))
  (bind _output_get (Variables|Default|SetCharacter _asbp_player_character))
  (if (Networking|IsServer)
    (EventDispatchers|AssignOnTakeAnyDamage _output_get (EventDispatchers|CreateEvent :!event Custom|OnPlayerTakeAnyDamage))))

(fn ApplyDamage
  (params (Damage :type Float%20%28single-precision%29))
  (bind _output_get (LocalVariables|SetL_Damage (|(Damage*(1-({1BF1DD35-4209-91C1-9D31-E0B2024BACCA}/200))) Damage)))
  (CallFunction|PrintMessage (Utilities|String|Append "Damage" (Utilities|String|ToString(Float) _output_get)) "(R=0.013012,G=1.000000,B=0.000000,A=1.000000)" 2.0 false)
  (Variables|Default|SetHealth (- (Variables|Default|GetHealth) (LocalVariables|GetL_Damage)))
  (Variables|Default|SetArmor (|(max(({1BF1DD35-4209-91C1-9D31-E0B2024BACCA}-({71A15CD0-403E-97B8-47E5-76A00244B8E0}*2)),0)))))

(fn GetHealth
  (return (Variables|Default|GetHealth) (Variables|Default|GetMaxHealth)))

(fn GetArmor
  (return (Variables|Default|GetArmor) (Variables|Default|GetMaxArmor)))