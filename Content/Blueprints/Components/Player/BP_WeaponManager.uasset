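; Player character component that spawns, stores and selects the character's weapons by type: main, secondary, special, grenade and melee.
; CreateWeapon spawns and files each weapon, then attaches it to the character.
; SelectWeapon sets CurrentWeapon, although its Grenade option reads the Specials array instead of Grenades.
; On clients, CurrentWeapon's OnRep moves the previous weapon back onto the character and attaches the new one to the visible mesh's weapon socket.
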(event `self.ReceiveBeginPlay`
  (bind _asbp_player_character (cast `/Game/Blueprints/Player/BP_PlayerCharacter` (`self.GetOwner`)))
  (set `self.Character` _asbp_player_character))

(event `SelectWeaponFromClient`
  (params (Type :type "/Game/Data/Enums/E_WeaponType Enum" :default "NewEnumerator0"))
  (`self.SelectWeapon` Type))

(fn `CreateWeapon`
  (params (Class :type "/Game/Blueprints/Weapons/BP_Weapon Class Reference"))
  (returns (Weapon :type "/Game/Blueprints/Weapons/BP_Weapon Object Reference"))
  (locals (L_Weapon :type "/Game/Blueprints/Weapons/BP_Weapon Object Reference"))
  (bind _character (`self.Character`))
  (bind _l_weapon (`local.L_Weapon`))
  (bind _returnvalue (`|SpawnActorFromClass` Class (`KismetMathLibrary.MakeTransform` (0.0 0.0 0.0)) "Undefined" "OverrideRootScale" (`Pawn.GetController` _character) _character))
  (bind _output_get (set `local.L_Weapon` _returnvalue))
  (switch `/Game/Data/Enums/E_WeaponType` (`/Game/Blueprints/Weapons/BP_Weapon.WeaponType` _output_get)
    (:`NewEnumerator0`
      (set `self.MainWeapon` _l_weapon))
    (:`NewEnumerator1`
      (set `self.SecondWeapon` _l_weapon))
    (:`NewEnumerator2`
      (`KismetArrayLibrary.Array_Add` (`self.Specials`) _l_weapon))
    (:`NewEnumerator3`
      (`KismetArrayLibrary.Array_Add` (`self.Grenades`) _l_weapon))
    (:`NewEnumerator4`
      (set `self.MeleeWeapon` _l_weapon)))
  (`Actor.K2_AttachToActor` (`local.L_Weapon`) (`self.Character`) "None" "SnapToTarget" "SnapToTarget" "KeepRelative" true)
  (return (`local.L_Weapon`)))

(fn `OnRep_CurrentWeapon`
  (if (not (`KismetSystemLibrary.IsServer`))
    (bind _clientweaponattached (`self.ClientWeaponAttached`)
      (:`then`
        (`Actor.K2_AttachToActor` _clientweaponattached (`self.Character`) "None" "SnapToTarget" "SnapToTarget" "KeepRelative" true))
      (:`else`
        _))
    (`Actor.K2_AttachToComponent` (`self.CurrentWeapon`) (`/Game/Blueprints/Player/BP_PlayerCharacter.GetVisibleMesh` (`self.Character`)) "Skt_Weapon" "KeepRelative" "KeepRelative" "KeepRelative" true)
    (set `self.ClientWeaponAttached` (`self.CurrentWeapon`))
    (`/Game/Blueprints/Libs/BP_Functions_Debug.PrintMessage` "Weapon Attached" (struct :`G` 0.924271 :`B` 1.0 :`A` 1.0) 3.0)))

(fn `SelectWeapon`
  (params (Type :type "/Game/Data/Enums/E_WeaponType Enum" :default "NewEnumerator0") (Index :type Integer))
  (returns (Weapon :type "/Game/Blueprints/Weapons/BP_Weapon Object Reference"))
  (bind _returnvalue (select `/Game/Data/Enums/E_WeaponType` Type :`NewEnumerator0` (`self.MainWeapon`) :`NewEnumerator1` (`self.SecondWeapon`) :`NewEnumerator2` (`|GetArrayItem` (`self.Specials`) Index) :`NewEnumerator3` (`|GetArrayItem` (`self.Specials`) Index) :`NewEnumerator4` (`self.MeleeWeapon`)))
  (`/Engine/EditorBlueprintResources/StandardMacros.IsValid` _returnvalue
    (:`Is Valid`
      (bind _output_get (set `self.CurrentWeapon` _returnvalue))
      (return _output_get))
    (:`Is Not Valid`
      (return (`self.CurrentWeapon`)))))